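; BP_Fireplace is an interactable fireplace in the DevTest gameplay objects that can be switched on and off.
; Interact calls the ToggleFireplaceState event, ignores the instigator and always returns true.
; The toggle flips IsActive, then sets or clears the Fire component's particle template and shows or hides the PointLight to match.
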(event Custom|ToggleFireplaceState
  (bind _output_get (Variables|Default|SetIsActive (not (Variables|Default|GetIsActive))))
  (Effects|Components|ParticleSystem|SetTemplate (Variables|Default|GetFire) (select _output_get "/Game/AlchemistsHouse/Assets/Particles/Fire.Fire" 0))
  (Rendering|SetVisibility (Variables|Default|GetPointLight) _output_get false))

(fn ConstructionScript
  (|CallParentFunction))

(fn Interact
  (params (Instigator :type Actor%20Object%20Reference))
  (CallFunction|ToggleFireplaceState)
  (return true))