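; BP_Pickup is an interactable chest that gives a single pickup to whoever interacts with it.
; The first interaction opens it, with a Timeline rotating the cover socket and setting IsOpen when finished.
; A later interaction sends PickupClass to the instigator via PickUpItemMessage, then marks the chest empty and destroys its Widget and Sphere components.
; Interact returns false once the open chest is empty.
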(event Custom|OpenChest
  (if (not (Audio|Components|Audio|IsPlaying (Variables|Default|GetTimeline)))
    (bind _alpha (Timeline|Timeline Play)
      (:Update
        (Transformation|SetRelativeRotation (Variables|Default|GetChestCoverRotationSocket) (Math|Rotator|Lerp(Rotator) "0, 0, 0" "0.000000,0.000000,-140.000000" _alpha) false false))
      (:Finished
        (Variables|Default|SetIsOpen true)))))

(event Custom|DeactivateChest
  (Variables|Default|SetIsEmpty true)
  (Components|DestroyComponent (Variables|Default|GetWidget)))

(fn ConstructionScript
  (|CallParentFunction))

(fn Interact
  (params (Instigator :type Actor%20Object%20Reference))
  (if (Variables|Default|GetIsOpen)
    (if (Variables|Default|GetIsEmpty)
      (return false)
      (else
        (Class|PlayerCharacterInterface|PickUpItem(Message) Instigator (Variables|Default|GetPickupClass))
        (CallFunction|DeactivateChest)
        (return true)))
    (else
      (CallFunction|OpenChest)
      (return true))))