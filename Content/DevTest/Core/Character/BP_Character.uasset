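; BP_Character is a character Blueprint that handles interaction with world objects and item pickup feedback.
; Capsule overlaps set the current InteractiveObjectBase and clear it when any such object leaves.
; PlayInteractiveMontage plays an animation on the mesh, storing whether it can be aborted and flagging it as playing until completion.
; PickUpItem asks BP_HUD on the first player controller to add a new notification.
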(event OnComponentBeginOverlap(CapsuleComponent)
  (params (OverlappedComponent :type Primitive%20Component%20Object%20Reference) (OtherActor :type Actor%20Object%20Reference) (OtherComp :type Primitive%20Component%20Object%20Reference) (OtherBodyIndex :type Integer) (bFromSweep :type Boolean) (SweepResult :type Hit%20Result%20Structure%20%28by%20ref%29))
  (bind _asinteractive_object_base (Utilities|Casting|CastToInteractiveObjectBase OtherActor))
  (Class|CharacterBase|SetInteractiveObject _asinteractive_object_base))

(event OnComponentEndOverlap(CapsuleComponent)
  (params (OverlappedComponent :type Primitive%20Component%20Object%20Reference) (OtherActor :type Actor%20Object%20Reference) (OtherComp :type Primitive%20Component%20Object%20Reference) (OtherBodyIndex :type Integer))
  (Utilities|Casting|CastToInteractiveObjectBase OtherActor)
  (Class|CharacterBase|ClearInteractiveObject))

(event EventPlayInteractiveMontage
  (params (Animation :type Anim%20Montage%20Object%20Reference) (CanBeAborted :type Boolean))
  (Variables|Default|SetIsInteractiveAnimationCanBeAborted CanBeAborted)
  (Variables|Default|SetIsInteractiveAnimationPlaying true)
  (Animation|Montage|PlayMontage (Variables|Character|GetMesh) Animation
    (:OnCompleted
      (Variables|Default|SetIsInteractiveAnimationPlaying false))))

(event EventPickUpItem
  (params (Item :type Object%20Class%20Reference))
  (bind _asbp_hud (Utilities|Casting|CastToBP_HUD (HUD|GetHUD (Game|GetPlayerController 0))))
  (Default|AddNewNotify _asbp_hud))

(fn ConstructionScript)